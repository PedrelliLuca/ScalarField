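; BP_InteractableCube is an interactable cube that toggles between a base and an inflated scale when a player interacts with it.
; An Interaction component's OnInteraction event flips CurrentScale, applies it as the actor scale and immediately ends the interactor's interaction.
; SetInteractionActionText keeps the prompt in sync, showing "Inflate" or "Deflate" at BeginPlay and after each toggle.
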(event OnInteraction(Interaction)
  (params (interactor :type Interactor%20Interface))
  (if (Class|KismetMathLibrary|EqualExactlyVectorVector (Variables|Default|GetCurrentScale) (Variables|Default|GetBaseScale))
    (Variables|Default|SetCurrentScale (Variables|Default|GetInflatedScale))
    (else
      (Variables|Default|SetCurrentScale (Variables|Default|GetBaseScale))))
  (Transformation|SetActorScale3D (Variables|Default|GetCurrentScale))
  (CallFunction|SetInteractionActionText)
  (Class|Interactor|EndInteraction interactor))

(event EventBeginPlay
  (Variables|Default|SetCurrentScale (Variables|Default|GetBaseScale))
  (CallFunction|SetInteractionActionText))

(event Collision|EventActorBeginOverlap
  (params (OtherActor :type Actor%20Object%20Reference)))

(event EventTick
  (params (DeltaSeconds :type Float%20%28single-precision%29)))

(fn ConstructionScript)

(fn SetInteractionActionText
  (if (Class|KismetMathLibrary|EqualExactlyVectorVector (Variables|Default|GetCurrentScale) (Variables|Default|GetBaseScale))
    (Class|InteractionComponent|SetInteractableActionText (Variables|Default|GetInteraction) (Utilities|Text|FormatText "Inflate"))
    (else
      (Class|InteractionComponent|SetInteractableActionText (Variables|Default|GetInteraction) (Utilities|Text|FormatText "Deflate")))))