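; Experimental heat map Blueprint that animates the look of a static mesh through a material.
; The construction script caches the mesh's bounding box and applies a dynamic M_Cells material instance.
; Tick drives that material's Alpha parameter with a time-based sine wave, smoothly oscillating between zero and one.
; Despite its name, DrawToRenderTarget only sets that scalar, and the stored bounds go unused here.
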(event Custom|DrawToRenderTarget
  (params (alpha :type Float%20%28double-precision%29))
  (Rendering|Material|SetScalarParameterValue (Variables|Default|Get_cellsMaterial) "Alpha" alpha :!class /Script/Engine.MaterialInstanceDynamic))

(event EventTick
  (params (DeltaSeconds :type Float%20%28single-precision%29))
  (CallFunction|DrawtoRenderTarget (+ (* (Math|Trig|Sin(Radians) (+ (* (Variables|Default|Get_timer) (Variables|Default|Get_frequency)) (Variables|Default|Get_phase))) (Variables|Default|Get_amplitude)) (Variables|Default|Get_offset)))
  (Variables|Default|Set_timer (+ DeltaSeconds (Variables|Default|Get_timer))))

(event EventBeginPlay
  (bind _returnvalue (Math|Trig|GetPI))
  (bind _returnvalue_2 (* _returnvalue 0.5))
  (Variables|Default|Set_timer 0.0)
  (Variables|Default|Set_frequency _returnvalue_2)
  (Variables|Default|Set_amplitude 0.5)
  (Variables|Default|Set_offset 0.5)
  (Variables|Default|Set_phase _returnvalue_2))

(fn ConstructionScript
  (bind _staticmesh (Variables|Default|GetStaticMesh))
  (bind _staticmesh_2 (Variables|/Script/Engine.StaticMeshComponent|GetStaticMesh _staticmesh))
  (bind _returnvalue (StaticMesh|GetBoundingBox _staticmesh_2))
  (bind (_min _max) (Utilities|Struct|BreakBox _returnvalue))
  (LocalVariables|SetboundingBoxMin _min)
  (LocalVariables|SetboundingBoxMax _max)
  (bind _returnvalue_2 (Rendering|Material|CreateDynamicMaterialInstance "/Game/Experiments/M_Cells.M_Cells" "None" "None" :!class /Script/Engine.KismetMaterialLibrary))
  (bind _output_get (Variables|Default|Set_cellsMaterial _returnvalue_2))
  (Rendering|Material|SetMaterial (Variables|Default|GetStaticMesh) 0 _output_get))